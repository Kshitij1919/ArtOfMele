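; BP_CombatComponent is a combat component that plays a sequence of attack montages on a supplied skeletal mesh.
; CustoMAttack looks up each AttackDetails entry in the AttackMappings map and plays the montage found, using CurrentAnimationMontageIndex to track position.
; Each montage completion increments the index and calls the event again, resetting the index once the list is exhausted.
; An unconnected delay-based loop, an empty event and an empty function remain unused.
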(event `CustoMAttack`
  (params (SkeletalMeshComp :type "SkeletalMeshComponent Object Reference") (AttackDetails :type "Array of AttackDetails Structure"))
  (bind _currentanimationmontageindex (`self.CurrentAnimationMontageIndex`))
  (bind (_value _returnvalue) (`BlueprintMapLibrary.Map_Find` (`self.AttackMappings`) (`|GetArrayItem` AttackDetails _currentanimationmontageindex)))
  (if (< _currentanimationmontageindex (`KismetArrayLibrary.Array_Length` AttackDetails))
    (if _returnvalue
      (`|PlayMontage` SkeletalMeshComp _value
        (:`OnCompleted`
          (`/Engine/EditorBlueprintResources/StandardMacros.IncrementInt` (`self.CurrentAnimationMontageIndex`)
            (:`  `
              (`self.CustoMAttack` SkeletalMeshComp AttackDetails))))))
    (else
      (set `self.CurrentAnimationMontageIndex` 0))))

(event `CustomMontageplaywithDelay`)

(fn `NewFunction`
  (params (NewParam :type "Array of AttackDetails Structure")))