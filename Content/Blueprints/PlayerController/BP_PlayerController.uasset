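; Player controller for a melee fighting character, turning Enhanced Input into movement, camera and punch and kick attacks.
; BeginPlay caches the player character, its BP_CombatComponent and skeletal mesh, then adds the IMC_CombatMappings context.
; Each attack input enters combat if needed, then passes target, side and type to the component's PerfromAttackSequence.
; Sprint switches locomotion to running only outside combat, returning to jogging on release.
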(event `self.ReceiveBeginPlay`
  (bind _returnvalue (`GameplayStatics.GetPlayerCharacter` 0))
  (bind _returnvalue_2 (`self.GetComponentByClass` (`self.PlayerControlledCharacter`) "/Script/Engine.SkeletalMeshComponent"))
  (bind _returnvalue_3 (pcsubsystem `EnhancedInputLocalPlayerSubsystem` self))
  (`|ExecutionSequence`
    (:`then_0`
      ;[1 0 0.9264 1 15] Getting chracter Variables
      (`/Engine/EditorBlueprintResources/StandardMacros.IsValid` _returnvalue
        (:`Is Valid`
          (bind _output_get (set `self.PlayerControlledCharacter` _returnvalue))
          (bind _returnvalue_4 (`self.GetComponentByClass` _output_get "/Game/Blueprints/Components/BP_CombatComponent.BP_CombatComponent_C"))
          (`/Engine/EditorBlueprintResources/StandardMacros.IsValid` _returnvalue_4
            (:`Is Valid`
              (set `self.PlayeControlledCharacter_CombatComponent` _returnvalue_4)
              (`/Engine/EditorBlueprintResources/StandardMacros.IsValid` _returnvalue_2
                (:`Is Valid`
                  (set `self.SkeletalMeshComponent` _returnvalue_2))))))))
    (:`then_1`
      ;[0.9744 0 1 1 15] Adding Mapping context
      (`/Engine/EditorBlueprintResources/StandardMacros.IsValid` _returnvalue_3
        (:`Is Valid`
          (`EnhancedInputSubsystemInterface.AddMappingContext` _returnvalue_3 "/Game/Input/Combat/IMC_CombatMappings.IMC_CombatMappings" 0 (struct)))))))

(event `EnhancedInput|/Game/Input/Combat/PunchActionMappings/IA_Cross`
  (params (ActionValue :type Boolean) (ElapsedSeconds :type "Float (double-precision)") (TriggeredSeconds :type "Float (double-precision)") (InputAction :type "InputAction Object Reference" :default "/Game/Input/Combat/PunchActionMappings/IA_Cross.IA_Cross"))
  ;[1 1 1 1 15] PUNCHES
  ;;[1 0.2754 0 1 15] Perfrom Attack CROSS
  (:`Triggered`
    (if (not (`BaseCombatComponent.bIsInCombat` (`self.PlayeControlledCharacter_CombatComponent`)))
      (`BaseCombatComponent.UpdateIsCharacterInCombat` (`self.PlayeControlledCharacter_CombatComponent`) true))
    (`BaseCombatComponent.PerfromAttackSequence` (`self.PlayeControlledCharacter_CombatComponent`) (`|MakeArray` (make `AttackDetails` "HEAD" "RIGHT" "CROSS")) (`self.SkeletalMeshComponent`))))

(event `EnhancedInput|/Game/Input/Combat/PunchActionMappings/IA_Jab`
  (params (ActionValue :type Boolean) (ElapsedSeconds :type "Float (double-precision)") (TriggeredSeconds :type "Float (double-precision)") (InputAction :type "InputAction Object Reference" :default "/Game/Input/Combat/PunchActionMappings/IA_Jab.IA_Jab"))
  ;[1 1 1 1 15] PUNCHES
  ;;[0 0.1557 1 1 15] Perfrom Attack JAB
  (:`Triggered`
    (if (not (`BaseCombatComponent.bIsInCombat` (`self.PlayeControlledCharacter_CombatComponent`)))
      (`BaseCombatComponent.UpdateIsCharacterInCombat` (`self.PlayeControlledCharacter_CombatComponent`) true))
    (`BaseCombatComponent.PerfromAttackSequence` (`self.PlayeControlledCharacter_CombatComponent`) (`|MakeArray` (make `AttackDetails` "HEAD")) (`self.SkeletalMeshComponent`))))

(event `EnhancedInput|/Game/Input/FreeRoam/IA_FR_Movement`
  (params (ActionValue :type "Vector2D Structure") (ElapsedSeconds :type "Float (double-precision)") (TriggeredSeconds :type "Float (double-precision)") (InputAction :type "InputAction Object Reference" :default "/Game/Input/FreeRoam/IA_FR_Movement.IA_FR_Movement"))
  (bind (_returnvalue_roll _returnvalue_pitch _returnvalue_yaw) (`KismetMathLibrary.BreakRotator` (`Pawn.GetControlRotation` (`self.PlayerControlledCharacter`))))
  (bind (_returnvalue_roll_2 _returnvalue_pitch_2 _returnvalue_yaw_2) (`KismetMathLibrary.BreakRotator` (`Pawn.GetControlRotation` (`self.PlayerControlledCharacter`))))
  ;[1 1 1 1 15] Player Movement
  (:`Triggered`
    (`|ExecutionSequence`
      (:`then_0`
        (`Pawn.AddMovementInput` (`self.PlayerControlledCharacter`) (`KismetMathLibrary.GetRightVector` (`KismetMathLibrary.MakeRotator` _returnvalue_roll_2 0.0 _returnvalue_yaw_2)) ActionValue_X false))
      (:`then_1`
        (`Pawn.AddMovementInput` (`self.PlayerControlledCharacter`) (`KismetMathLibrary.GetForwardVector` (`KismetMathLibrary.MakeRotator` 0.0 0.0 _returnvalue_yaw)) ActionValue_Y false)))))

(event `EnhancedInput|/Game/Input/Combat/PunchActionMappings/IA_LeftHook`
  (params (ActionValue :type Boolean) (ElapsedSeconds :type "Float (double-precision)") (TriggeredSeconds :type "Float (double-precision)") (InputAction :type "InputAction Object Reference" :default "/Game/Input/Combat/PunchActionMappings/IA_LeftHook.IA_LeftHook"))
  ;[1 1 1 1 15] PUNCHES
  ;;[0 1 0.0966 1 15] Perfrom Attack LEFT HOOK
  (:`Triggered`
    (if (not (`BaseCombatComponent.bIsInCombat` (`self.PlayeControlledCharacter_CombatComponent`)))
      (`BaseCombatComponent.UpdateIsCharacterInCombat` (`self.PlayeControlledCharacter_CombatComponent`) true))
    (`BaseCombatComponent.PerfromAttackSequence` (`self.PlayeControlledCharacter_CombatComponent`) (`|MakeArray` (make `AttackDetails` "HEAD" "LEFT" "HOOK")) (`self.SkeletalMeshComponent`))))

(event `EnhancedInput|/Game/Input/Combat/PunchActionMappings/IA_RightHook`
  (params (ActionValue :type Boolean) (ElapsedSeconds :type "Float (double-precision)") (TriggeredSeconds :type "Float (double-precision)") (InputAction :type "InputAction Object Reference" :default "/Game/Input/Combat/PunchActionMappings/IA_RightHook.IA_RightHook"))
  ;[1 1 1 1 15] PUNCHES
  ;;[1 0 0 1 15] Perfrom Attack RIGHT HOOK
  (:`Triggered`
    (if (not (`BaseCombatComponent.bIsInCombat` (`self.PlayeControlledCharacter_CombatComponent`)))
      (`BaseCombatComponent.UpdateIsCharacterInCombat` (`self.PlayeControlledCharacter_CombatComponent`) true))
    (`BaseCombatComponent.PerfromAttackSequence` (`self.PlayeControlledCharacter_CombatComponent`) (`|MakeArray` (make `AttackDetails` "HEAD" "RIGHT" "HOOK")) (`self.SkeletalMeshComponent`))))

(event `EnhancedInput|/Game/Input/FreeRoam/IA_CameraRotation`
  (params (ActionValue :type "Vector2D Structure") (ElapsedSeconds :type "Float (double-precision)") (TriggeredSeconds :type "Float (double-precision)") (InputAction :type "InputAction Object Reference" :default "/Game/Input/FreeRoam/IA_CameraRotation.IA_CameraRotation"))
  ;[1 1 1 1 15] Camera Rotaion
  (:`Triggered`
    (`|ExecutionSequence`
      (:`then_0`
        (`Pawn.AddControllerYawInput` (`self.PlayerControlledCharacter`) ActionValue_X))
      (:`then_1`
        (`Pawn.AddControllerPitchInput` (`self.PlayerControlledCharacter`) ActionValue_Y)))))

(event `EnhancedInput|/Game/Input/Combat/PunchActionMappings/IA_BodyCross`
  (params (ActionValue :type Boolean) (ElapsedSeconds :type "Float (double-precision)") (TriggeredSeconds :type "Float (double-precision)") (InputAction :type "InputAction Object Reference" :default "/Game/Input/Combat/PunchActionMappings/IA_BodyCross.IA_BodyCross"))
  ;[1 1 1 1 15] PUNCHES
  ;;[0 0 0 1 15] Body Punch Attacks
  ;;;[1 0.2754 0 1 15] Perfrom Attack BODY CROSS
  (:`Triggered`
    (if (not (`BaseCombatComponent.bIsInCombat` (`self.PlayeControlledCharacter_CombatComponent`)))
      (`BaseCombatComponent.UpdateIsCharacterInCombat` (`self.PlayeControlledCharacter_CombatComponent`) true))
    (`BaseCombatComponent.PerfromAttackSequence` (`self.PlayeControlledCharacter_CombatComponent`) (`|MakeArray` (make `AttackDetails` "BODY" "RIGHT" "CROSS")) (`self.SkeletalMeshComponent`))))

(event `EnhancedInput|/Game/Input/Combat/PunchActionMappings/IA_BodyJab`
  (params (ActionValue :type Boolean) (ElapsedSeconds :type "Float (double-precision)") (TriggeredSeconds :type "Float (double-precision)") (InputAction :type "InputAction Object Reference" :default "/Game/Input/Combat/PunchActionMappings/IA_BodyJab.IA_BodyJab"))
  ;[1 1 1 1 15] PUNCHES
  ;;[0 0 0 1 15] Body Punch Attacks
  ;;;[0 0.1557 1 1 15] Perfrom Attack BODY JAB
  (:`Triggered`
    (if (not (`BaseCombatComponent.bIsInCombat` (`self.PlayeControlledCharacter_CombatComponent`)))
      (`BaseCombatComponent.UpdateIsCharacterInCombat` (`self.PlayeControlledCharacter_CombatComponent`) true))
    (`BaseCombatComponent.PerfromAttackSequence` (`self.PlayeControlledCharacter_CombatComponent`) (`|MakeArray` (make `AttackDetails` "BODY")) (`self.SkeletalMeshComponent`))))

(event `EnhancedInput|/Game/Input/Combat/IA_SpecialAttackModifier_Sprint`
  (params (ActionValue :type Boolean) (ElapsedSeconds :type "Float (double-precision)") (TriggeredSeconds :type "Float (double-precision)") (InputAction :type "InputAction Object Reference" :default "/Game/Input/Combat/IA_SpecialAttackModifier_Sprint.IA_SpecialAttackModifier_Sprint"))
  ;[1 1 1 1 15] Sprint or Special Attack
  (:`Started`
    (if (not (`BaseCombatComponent.bIsInCombat` (`self.PlayeControlledCharacter_CombatComponent`)))
      (message `CharacterInterface.UpdateCharacterLocomotionState` (`self.PlayerControlledCharacter`) "RUNNING")))
  (:`Completed`
    (message `CharacterInterface.UpdateCharacterLocomotionState` (`self.PlayerControlledCharacter`) "JOGGING")))

(event `EnhancedInput|/Game/Input/Combat/PunchActionMappings/IA_LeftBodyHook`
  (params (ActionValue :type Boolean) (ElapsedSeconds :type "Float (double-precision)") (TriggeredSeconds :type "Float (double-precision)") (InputAction :type "InputAction Object Reference" :default "/Game/Input/Combat/PunchActionMappings/IA_LeftBodyHook.IA_LeftBodyHook"))
  ;[1 1 1 1 15] PUNCHES
  ;;[0 0 0 1 15] Body Punch Attacks
  ;;;[0 1 0.0966 1 15] Perfrom Attack BODY LEFT HOOK
  (:`Triggered`
    (if (not (`BaseCombatComponent.bIsInCombat` (`self.PlayeControlledCharacter_CombatComponent`)))
      (`BaseCombatComponent.UpdateIsCharacterInCombat` (`self.PlayeControlledCharacter_CombatComponent`) true))
    (`BaseCombatComponent.PerfromAttackSequence` (`self.PlayeControlledCharacter_CombatComponent`) (`|MakeArray` (make `AttackDetails` "BODY" "LEFT" "HOOK")) (`self.SkeletalMeshComponent`))))

(event `EnhancedInput|/Game/Input/Combat/PunchActionMappings/IA_RightBodyHook`
  (params (ActionValue :type Boolean) (ElapsedSeconds :type "Float (double-precision)") (TriggeredSeconds :type "Float (double-precision)") (InputAction :type "InputAction Object Reference" :default "/Game/Input/Combat/PunchActionMappings/IA_RightBodyHook.IA_RightBodyHook"))
  ;[1 1 1 1 15] PUNCHES
  ;;[0 0 0 1 15] Body Punch Attacks
  ;;;[1 0 0 1 15] Perfrom Attack BODY RIGHT HOOK
  (:`Triggered`
    (if (not (`BaseCombatComponent.bIsInCombat` (`self.PlayeControlledCharacter_CombatComponent`)))
      (`BaseCombatComponent.UpdateIsCharacterInCombat` (`self.PlayeControlledCharacter_CombatComponent`) true))
    (`BaseCombatComponent.PerfromAttackSequence` (`self.PlayeControlledCharacter_CombatComponent`) (`|MakeArray` (make `AttackDetails` "BODY" "RIGHT" "HOOK")) (`self.SkeletalMeshComponent`))))

(event `EnhancedInput|/Game/Input/Combat/KickActionMappings/IA_FrontRightKick`
  (params (ActionValue :type Boolean) (ElapsedSeconds :type "Float (double-precision)") (TriggeredSeconds :type "Float (double-precision)") (InputAction :type "InputAction Object Reference" :default "/Game/Input/Combat/KickActionMappings/IA_FrontRightKick.IA_FrontRightKick"))
  ;[1 1 1 1 15] KICKS
  ;;[1 0.2754 0 1 15] Perfrom Attack FRONT RIGHT KICK
  (:`Triggered`
    (if (not (`BaseCombatComponent.bIsInCombat` (`self.PlayeControlledCharacter_CombatComponent`)))
      (`BaseCombatComponent.UpdateIsCharacterInCombat` (`self.PlayeControlledCharacter_CombatComponent`) true))
    (`BaseCombatComponent.PerfromAttackSequence` (`self.PlayeControlledCharacter_CombatComponent`) (`|MakeArray` (make `AttackDetails` "HEAD" "RIGHT" "FRONTKICK")) (`self.SkeletalMeshComponent`))))

(event `EnhancedInput|/Game/Input/Combat/KickActionMappings/IA_FrontLeftKick`
  (params (ActionValue :type Boolean) (ElapsedSeconds :type "Float (double-precision)") (TriggeredSeconds :type "Float (double-precision)") (InputAction :type "InputAction Object Reference" :default "/Game/Input/Combat/KickActionMappings/IA_FrontLeftKick.IA_FrontLeftKick"))
  ;[1 1 1 1 15] KICKS
  ;;[0 0.1557 1 1 15] Perfrom Attack FRONT LEFT KICK
  (:`Triggered`
    (if (not (`BaseCombatComponent.bIsInCombat` (`self.PlayeControlledCharacter_CombatComponent`)))
      (`BaseCombatComponent.UpdateIsCharacterInCombat` (`self.PlayeControlledCharacter_CombatComponent`) true))
    (`BaseCombatComponent.PerfromAttackSequence` (`self.PlayeControlledCharacter_CombatComponent`) (`|MakeArray` (make `AttackDetails` "HEAD" "LEFT" "FRONTKICK")) (`self.SkeletalMeshComponent`))))

(event `EnhancedInput|/Game/Input/Combat/KickActionMappings/IA_LeftHeadKick`
  (params (ActionValue :type Boolean) (ElapsedSeconds :type "Float (double-precision)") (TriggeredSeconds :type "Float (double-precision)") (InputAction :type "InputAction Object Reference" :default "/Game/Input/Combat/KickActionMappings/IA_LeftHeadKick.IA_LeftHeadKick"))
  ;[1 1 1 1 15] KICKS
  ;;[0 1 0.0966 1 15] Perfrom Attack LEFT HEAD KICK
  (:`Triggered`
    (if (not (`BaseCombatComponent.bIsInCombat` (`self.PlayeControlledCharacter_CombatComponent`)))
      (`BaseCombatComponent.UpdateIsCharacterInCombat` (`self.PlayeControlledCharacter_CombatComponent`) true))
    (`BaseCombatComponent.PerfromAttackSequence` (`self.PlayeControlledCharacter_CombatComponent`) (`|MakeArray` (make `AttackDetails` "HEAD" "LEFT" "ROUNDHOUSEKICK")) (`self.SkeletalMeshComponent`))))

(event `EnhancedInput|/Game/Input/Combat/KickActionMappings/IA_RightHeadKick`
  (params (ActionValue :type Boolean) (ElapsedSeconds :type "Float (double-precision)") (TriggeredSeconds :type "Float (double-precision)") (InputAction :type "InputAction Object Reference" :default "/Game/Input/Combat/KickActionMappings/IA_RightHeadKick.IA_RightHeadKick"))
  ;[1 1 1 1 15] KICKS
  ;;[1 0 0 1 15] Perfrom Attack RIGHT HEAD KICK
  (:`Triggered`
    (if (not (`BaseCombatComponent.bIsInCombat` (`self.PlayeControlledCharacter_CombatComponent`)))
      (`BaseCombatComponent.UpdateIsCharacterInCombat` (`self.PlayeControlledCharacter_CombatComponent`) true))
    (`BaseCombatComponent.PerfromAttackSequence` (`self.PlayeControlledCharacter_CombatComponent`) (`|MakeArray` (make `AttackDetails` "HEAD" "RIGHT" "ROUNDHOUSEKICK")) (`self.SkeletalMeshComponent`))))

(event `EnhancedInput|/Game/Input/Combat/KickActionMappings/IA_FrontRightBodyKick`
  (params (ActionValue :type Boolean) (ElapsedSeconds :type "Float (double-precision)") (TriggeredSeconds :type "Float (double-precision)") (InputAction :type "InputAction Object Reference" :default "/Game/Input/Combat/KickActionMappings/IA_FrontRightBodyKick.IA_FrontRightBodyKick"))
  ;[1 1 1 1 15] KICKS
  ;;[0 0 0 1 15] Body Kick Attacks
  ;;;[1 0.2754 0 1 15] Perfrom Attack FRONT RIGHT BODY KICK
  (:`Triggered`
    (if (not (`BaseCombatComponent.bIsInCombat` (`self.PlayeControlledCharacter_CombatComponent`)))
      (`BaseCombatComponent.UpdateIsCharacterInCombat` (`self.PlayeControlledCharacter_CombatComponent`) true))
    (`BaseCombatComponent.PerfromAttackSequence` (`self.PlayeControlledCharacter_CombatComponent`) (`|MakeArray` (make `AttackDetails` "BODY" "RIGHT" "FRONTKICK")) (`self.SkeletalMeshComponent`))))

(event `EnhancedInput|/Game/Input/Combat/KickActionMappings/IA_FrontLeftBodyKick`
  (params (ActionValue :type Boolean) (ElapsedSeconds :type "Float (double-precision)") (TriggeredSeconds :type "Float (double-precision)") (InputAction :type "InputAction Object Reference" :default "/Game/Input/Combat/KickActionMappings/IA_FrontLeftBodyKick.IA_FrontLeftBodyKick"))
  ;[1 1 1 1 15] KICKS
  ;;[0 0 0 1 15] Body Kick Attacks
  ;;;[0 0.1557 1 1 15] Perfrom Attack FRONT LEFT BODY KICK
  (:`Triggered`
    (if (not (`BaseCombatComponent.bIsInCombat` (`self.PlayeControlledCharacter_CombatComponent`)))
      (`BaseCombatComponent.UpdateIsCharacterInCombat` (`self.PlayeControlledCharacter_CombatComponent`) true))
    (`BaseCombatComponent.PerfromAttackSequence` (`self.PlayeControlledCharacter_CombatComponent`) (`|MakeArray` (make `AttackDetails` "BODY" "LEFT" "FRONTKICK")) (`self.SkeletalMeshComponent`))))

(event `EnhancedInput|/Game/Input/Combat/KickActionMappings/IA_LeftBodyKick`
  (params (ActionValue :type Boolean) (ElapsedSeconds :type "Float (double-precision)") (TriggeredSeconds :type "Float (double-precision)") (InputAction :type "InputAction Object Reference" :default "/Game/Input/Combat/KickActionMappings/IA_LeftBodyKick.IA_LeftBodyKick"))
  ;[1 1 1 1 15] KICKS
  ;;[0 0 0 1 15] Body Kick Attacks
  ;;;[0 1 0.0966 1 15] Perfrom Attack LEFT BODY KICK
  (:`Triggered`
    (if (not (`BaseCombatComponent.bIsInCombat` (`self.PlayeControlledCharacter_CombatComponent`)))
      (`BaseCombatComponent.UpdateIsCharacterInCombat` (`self.PlayeControlledCharacter_CombatComponent`) true))
    (`BaseCombatComponent.PerfromAttackSequence` (`self.PlayeControlledCharacter_CombatComponent`) (`|MakeArray` (make `AttackDetails` "BODY" "LEFT" "ROUNDHOUSEKICK")) (`self.SkeletalMeshComponent`))))

(event `EnhancedInput|/Game/Input/Combat/KickActionMappings/IA_RightBodyKick`
  (params (ActionValue :type Boolean) (ElapsedSeconds :type "Float (double-precision)") (TriggeredSeconds :type "Float (double-precision)") (InputAction :type "InputAction Object Reference" :default "/Game/Input/Combat/KickActionMappings/IA_RightBodyKick.IA_RightBodyKick"))
  ;[1 1 1 1 15] KICKS
  ;;[0 0 0 1 15] Body Kick Attacks
  ;;;[1 0 0 1 15] Perfrom Attack RIGHT BODY KICK
  (:`Triggered`
    (if (not (`BaseCombatComponent.bIsInCombat` (`self.PlayeControlledCharacter_CombatComponent`)))
      (`BaseCombatComponent.UpdateIsCharacterInCombat` (`self.PlayeControlledCharacter_CombatComponent`) true))
    (`BaseCombatComponent.PerfromAttackSequence` (`self.PlayeControlledCharacter_CombatComponent`) (`|MakeArray` (make `AttackDetails` "BODY" "RIGHT" "ROUNDHOUSEKICK")) (`self.SkeletalMeshComponent`))))

(fn `UserConstructionScript`)